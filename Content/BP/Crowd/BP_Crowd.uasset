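; BP_Crowd is a crowd actor that slides along the world Y axis shortly after play begins.
; On BeginPlay it stores its root location and the absolute Y distance to Ypostarget, then waits briefly before starting a timeline.
; The timeline's Crowdpos track scales that distance as an offset added to the starting Y, keeping X and Z fixed.
; Because the distance is absolute, the target's side does not affect the offset's sign.
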(event EventBeginPlay
  (bind _defaultsceneroot (Variables|Default|GetDefaultSceneRoot))
  (Variables|Default|SetPos (Transformation|GetWorldLocation _defaultsceneroot))
  (Variables|Default|SetDistance (Math|Float|Absolute(Float) (- (.y (Variables|Default|GetPos)) (Variables|Default|GetYpostarget))))
  (Utilities|FlowControl|Delay 2.0)
  (bind _crowdpos (Timeline|Timeline Play)
    (:Update
      (Transformation|SetWorldLocation _defaultsceneroot (Math|Vector|MakeVector (.x (Variables|Default|GetPos)) (+ (.y (Variables|Default|GetPos)) (* _crowdpos (Variables|Default|GetDistance))) (.z (Variables|Default|GetPos))) false false))))

(fn ConstructionScript)