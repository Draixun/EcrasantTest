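; Demon monster that stalks the player along the Y axis, raising their Anxiete by Damage when its approach completes.
; The GettingCloser timeline drives AI moves from an offset in front or behind, set by Backward, toward the player.
; Being flashed stops the approach and sends it back; the timeline restarts after a delay following either outcome.
; Tick keeps it facing the player and teleports it to that offset when too far away.
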(event Custom|Flashed
  (bind _returnvalue (Transformation|GetActorLocation))
  (bind _returnvalue_2 (Transformation|GetActorLocation))
  (bind _as_bp_third_person_character (Variables|Default|GetAs%20BP%20Third%20Person%20Character))
  (bind _max_value_y (Variables|Default|GetMax%20Value%20Y))
  (bind _player_value_y (Variables|Default|GetPlayer%20Value%20Y))
  (Utilities|FlowControl|Sequence
    (:then_0
      (bind _position (Timeline|Getting%20closer Stop)
        (:Update
          (if (Variables|Default|GetBackward?)
            (Variables|Default|SetTarget_pos (+ _max_value_y _player_value_y))
            (else
              (Variables|Default|SetTarget_pos (+ (* _max_value_y -1.0) _player_value_y))))
          (AI|AIMoveTo self (Math|Vector|MakeVector (.x _returnvalue_2) (Math|Float|Lerp (Variables|Default|GetTarget_pos) (Variables|Default|GetPlayer%20Value%20Y) _position) (.z _returnvalue_2)) 0 1.0 false))
        (:Finished
          (if (== _position 1.0) :!label _label
            (Utilities|FlowControl|DoOnce false :!label _label_2
              (:Completed
                (Variables|/Game/ThirdPerson/Blueprints/BP_ThirdPersonCharacter.BP_ThirdPersonCharacter_C|SetAnxiete _as_bp_third_person_character (+ (Variables|/Game/ThirdPerson/Blueprints/BP_ThirdPersonCharacter.BP_ThirdPersonCharacter_C|GetAnxiete _as_bp_third_person_character) (Variables|Default|GetDamage))))))
          (Utilities|FlowControl|Sequence
            (:then_0
              (Timeline|Getting%20closer Stop))
            (:then_1
              (Utilities|FlowControl|Delay 3.0)
              (Utilities|FlowControl|Sequence
                (:then_0
                  (Timeline|Getting%20closer PlayFromStart))
                (:then_1
                  (goto _label_2 Reset))))))))
    (:then_1
      (AI|AIMoveTo self (Math|Vector|MakeVector (.x _returnvalue) (Variables|Default|GetBACKPOS) (.z _returnvalue)) 0 1.0 false
        (:then
          (goto _label))))))

(event Custom|Set_Mesh)

(event EventBeginPlay
  (bind _returnvalue (Transformation|GetActorLocation))
  (bind _max_value_y (Variables|Default|GetMax%20Value%20Y))
  (bind _player_value_y (Variables|Default|GetPlayer%20Value%20Y))
  (bind _asbp_third_person_character (Utilities|Casting|CastToBP_ThirdPersonCharacter (Game|GetPlayerCharacter 0)))
  (Variables|Default|SetAs%20BP%20Third%20Person%20Character _asbp_third_person_character)
  (Variables|Default|SetMesh_offset (Math|Float|Absolute(Float) (- (.x (Transformation|GetWorldLocation (Variables|Character|GetMesh))) (.x (Transformation|GetActorLocation)))))
  (bind _position (Timeline|Getting%20closer PlayFromStart)
    (:Update
      (if (Variables|Default|GetBackward?)
        (Variables|Default|SetTarget_pos (+ _max_value_y _player_value_y))
        (else
          (Variables|Default|SetTarget_pos (+ (* _max_value_y -1.0) _player_value_y))))
      (AI|AIMoveTo self (Math|Vector|MakeVector (.x _returnvalue) (Math|Float|Lerp (Variables|Default|GetTarget_pos) (Variables|Default|GetPlayer%20Value%20Y) _position) (.z _returnvalue)) 0 1.0 false))
    (:Finished
      (if (== _position 1.0)
        (Utilities|FlowControl|DoOnce false :!label _label
          (:Completed
            (Variables|/Game/ThirdPerson/Blueprints/BP_ThirdPersonCharacter.BP_ThirdPersonCharacter_C|SetAnxiete (Variables|Default|GetAs%20BP%20Third%20Person%20Character) (+ (Variables|/Game/ThirdPerson/Blueprints/BP_ThirdPersonCharacter.BP_ThirdPersonCharacter_C|GetAnxiete (Variables|Default|GetAs%20BP%20Third%20Person%20Character)) (Variables|Default|GetDamage))))))
      (Utilities|FlowControl|Sequence
        (:then_0
          (Timeline|Getting%20closer Stop))
        (:then_1
          (Utilities|FlowControl|Delay 3.0)
          (Utilities|FlowControl|Sequence
            (:then_0
              (Timeline|Getting%20closer PlayFromStart))
            (:then_1
              (goto _label Reset))))))))

(event Collision|EventActorBeginOverlap
  (params (OtherActor :type Actor%20Object%20Reference)))

(event EventTick
  (params (DeltaSeconds :type Float%20%28single-precision%29))
  (bind _returnvalue (Transformation|GetActorLocation))
  (bind (_x _y _z) (Class|KismetMathLibrary|BreakVector3f _returnvalue))
  (Variables|Default|SetPlayer%20Value%20Y (.y (Transformation|GetActorLocation (Variables|Default|GetAs%20BP%20Third%20Person%20Character))))
  (Variables|Default|SetMonster%20Value%20Y (.y (Transformation|GetActorLocation)))
  (Utilities|SetBackpos)
  (if (> (Math|Float|Absolute(Float) (- (Variables|Default|GetPlayer%20Value%20Y) (Variables|Default|GetMonster%20Value%20Y))) (Variables|Default|GetMax%20Value%20Y))
    (Utilities|StayinScreen))
  (Transformation|SetActorRotation (Math|Rotator|FindLookatRotation _returnvalue (Math|Vector|MakeVector _x (Variables|Default|GetPlayer%20Value%20Y) _z))))

(fn ConstructionScript)