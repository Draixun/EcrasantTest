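; BP_Demon is an enemy that chases the player and raises their Anxiete at close range, printing "Dead" at the maximum.
; Tick drives AIMoveTo; contact triggers cooldown-limited damage and a self-stun that pauses or, when Underground, slows it.
; Vanish runs a timeline on the Parameter_Demon collection's dissolve amount, then reverses it; dissolving blocks attacks and stuns.
; Underground also alters damage, dissolve depth and collision disabling.
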(event Custom|Vanish
  (bind _capsulecomponent (Variables|Collision|GetCapsuleComponent))
  ;[1 1 1] Vnish Effect
  (bind _returnvalue (Rendering|Material|GetScalarParameterValue "/Game/Art/Collection/Parameter_Demon.Parameter_Demon" "Dissolve_Amount" :!class /Script/Engine.KismetMaterialLibrary))
  (if (< _returnvalue 0.05)
    (if (Variables|Default|GetUnderground)
      (bind _dissolveamount (Timeline|Dissolve%20effect Play)
        (:Update
          (if (Variables|Default|GetUnderground)
            (Rendering|Material|SetScalarParameterValue "/Game/Art/Collection/Parameter_Demon.Parameter_Demon" "Dissolve_Amount" (* _dissolveamount 0.5) :!class /Script/Engine.KismetMaterialLibrary)
            (else
              (Rendering|Material|SetScalarParameterValue "/Game/Art/Collection/Parameter_Demon.Parameter_Demon" "Dissolve_Amount" _dissolveamount :!class /Script/Engine.KismetMaterialLibrary))))
        (:Finished
          (if (> _dissolveamount 0.1)
            (Utilities|FlowControl|Delay 1.0)
            (Collision|SetCollisionEnabled _capsulecomponent "QueryAndPhysics")
            (Timeline|Dissolve%20effect Reverse))))
      (else
        (Collision|SetCollisionEnabled _capsulecomponent "NoCollision")
        (Timeline|Dissolve%20effect Play)))))

(event Custom|Stunned
  (bind _self self)
  (bind _charactermovement (Variables|Character|GetCharacterMovement))
  ;[1 1 1] Stun
  (bind _returnvalue (Rendering|Material|GetScalarParameterValue "/Game/Art/Collection/Parameter_Demon.Parameter_Demon" "Dissolve_Amount" :!class /Script/Engine.KismetMaterialLibrary))
  (if (< _returnvalue 0.05)
    (if (Variables|Default|GetUnderground)
      (Variables|/Script/Engine.CharacterMovementComponent|SetMaxWalkSpeed _charactermovement 1.5e+02)
      (Utilities|FlowControl|Delay 6.0)
      (Variables|/Script/Engine.CharacterMovementComponent|SetMaxWalkSpeed _charactermovement 5e+02)
      (else
        (AI|AIMoveTo _self "0, 0, 0" _self 5.0 false
          (:then
            (Variables|Default|SetIsStun? true)
            (Utilities|FlowControl|Delay 2.0)
            (Variables|Default|SetIsStun? false)))))))

(event EventTick
  (params (DeltaSeconds :type Float%20%28single-precision%29))
  (bind _playerref (Variables|Default|GetPlayerRef))
  ;[1 1 1] Behaviour
  (if (not (Variables|Default|GetIsStun?))
    (AI|AIMoveTo self "0, 0, 0" (Variables|Default|GetPlayerRef) 5.0 false
      (:then
        (bind _returnvalue (Rendering|Material|GetScalarParameterValue "/Game/Art/Collection/Parameter_Demon.Parameter_Demon" "Dissolve_Amount" :!class /Script/Engine.KismetMaterialLibrary))
        (if (and (<= (Math|Vector|VectorLengthXY (- (Transformation|GetActorLocation) (Transformation|GetActorLocation (Variables|Default|GetPlayerRef)))) 8e+01) (<= _returnvalue 0.0))
          ;[1 1 1] Damage
          (CallFunction|Stunned)
          (Utilities|FlowControl|DoOnce false :!label _label
            (:Completed
              (if (Variables|Default|GetUnderground)
                (Variables|/Game/ThirdPerson/Blueprints/BP_ThirdPersonCharacter.BP_ThirdPersonCharacter_C|SetAnxiete _playerref (+ (Variables|/Game/ThirdPerson/Blueprints/BP_ThirdPersonCharacter.BP_ThirdPersonCharacter_C|GetAnxiete _playerref) (Variables|Default|GetDemon_Damage)))
                (else
                  (Variables|/Game/ThirdPerson/Blueprints/BP_ThirdPersonCharacter.BP_ThirdPersonCharacter_C|SetAnxiete _playerref (/ (+ (Variables|/Game/ThirdPerson/Blueprints/BP_ThirdPersonCharacter.BP_ThirdPersonCharacter_C|GetAnxiete _playerref) (Variables|Default|GetDemon_Damage)) 4.0))))
              (if (>= (Variables|/Game/ThirdPerson/Blueprints/BP_ThirdPersonCharacter.BP_ThirdPersonCharacter_C|GetAnxiete _playerref) (Variables|/Game/ThirdPerson/Blueprints/BP_ThirdPersonCharacter.BP_ThirdPersonCharacter_C|GetAnxiete_max _playerref))
                (Utilities|FlowControl|DoOnce false
                  (:Completed
                    (Development|PrintString "Dead" true true "(R=1.000000,G=0.000000,B=0.028078,A=1.000000)")))
                (else
                  (Utilities|FlowControl|Delay 2.0)
                  (goto _label Reset))))))))))

(event EventBeginPlay
  (bind _mesh (Variables|Character|GetMesh))
  (bind _asbp_third_person_character (Utilities|Casting|CastToBP_ThirdPersonCharacter (Game|GetPlayerCharacter 0)))
  (Variables|Default|SetPlayerRef _asbp_third_person_character)
  (Components|Animation|PlayAnimation (Variables|Character|GetMesh) "/Game/Art/Model/Chara/Monster/monster_rigged_Skeleton_Sequence_mouth.monster_rigged_Skeleton_Sequence_mouth" true)
  (Components|Timeline|SetPlayRate _mesh 1.0 :!label _label)
  (Utilities|FlowControl|Delay 0.5)
  (Components|Timeline|SetPlayRate _mesh -1.0)
  (Utilities|FlowControl|Delay 0.5)
  (goto _label))

(fn ConstructionScript)