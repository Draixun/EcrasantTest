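; Bird actor that takes flight when the third-person character overlaps it.
; On overlap it computes a target from its start position along a direction scaled by Speed, then sets its child skeletal meshes to a looping fly animation, yawed toward that target.
; A Timeline lerps the whole actor from start to target without sweep.
; The Get_Direction graph holds only an unconnected target-minus-start calculation.
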(event EventTick
  (params (DeltaSeconds :type Float%20%28single-precision%29)))

(event Collision|EventActorBeginOverlap
  (params (OtherActor :type Actor%20Object%20Reference))
  (Utilities|Casting|CastToBP_ThirdPersonCharacter OtherActor)
  (Variables|Default|SetStartPos (Transformation|GetActorLocation))
  (Variables|Default|SetIsFlying true)
  (Variables|Default|SetTargetPos (+ (* (Utilities|GetDirection) (Variables|Default|Getspeed)) (Variables|Default|GetStartPos)))
  (for _array_element (Components|GetChildrenComponents (Variables|Default|GetDefaultSceneRoot) false)
    (bind _asskeletal_mesh_component (Utilities|Casting|CastToSkeletalMeshComponent _array_element))
    (Components|Animation|PlayAnimation _asskeletal_mesh_component "/Game/Art/Model/corbeau/Bird_fly.Bird_fly" true)
    (Transformation|SetWorldRotation _asskeletal_mesh_component (Math|Rotator|MakeRotator 0.0 0.0 (.yaw (Class|KismetMathLibrary|QuatRotator (Math|Conversions|ToQuaternion(Rotator) (Math|Vector|Normalize (- (Variables|Default|GetTargetPos) (Variables|Default|GetStartPos))))))) false false)
    (bind _alpha (Timeline|Timeline Play)
      (:Update
        (Transformation|SetActorLocation (Math|Vector|Lerp(Vector) (Variables|Default|GetStartPos) (Variables|Default|GetTargetPos) _alpha) false false)))))

(fn ConstructionScript)