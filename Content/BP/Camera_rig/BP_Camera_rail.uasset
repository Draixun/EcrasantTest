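; Rail camera actor that moves the third-person character's follow camera along the first CameraRig_Rail found in the level.
; BeginPlay caches the rail spline and its end-point Y values, then detaches FollowCamera from the character.
; Each Tick treats the player mesh's world Y, relative to the first point's local Y, as spline distance, then places the camera there with a fixed world-Y offset and yaw correction.
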(event EventBeginPlay
  (bind _returnvalue (Actor|GetActorOfClass "/Script/CinematicCamera.CameraRig_Rail"))
  (bind _output_get (Variables|Default|SetRail_ref _returnvalue))
  (Variables|Default|SetSpline_ref (Class|CameraRigRail|GetRailSplineComponent _output_get))
  (bind _output_get_2 (Variables|Default|SetEnd%20Value%20Y (.y (Spline|GetLocationatSplinePoint (Class|CameraRigRail|GetRailSplineComponent _output_get) 0 "Local"))))
  (bind _output_get_3 (Variables|Default|SetStart%20Value%20Y (.y (Spline|GetLocationatSplinePoint (Class|CameraRigRail|GetRailSplineComponent _output_get) (- (Spline|GetNumberOfSplinePoints (Class|CameraRigRail|GetRailSplineComponent _output_get)) 1) "World"))))
  (Variables|Default|SetLenghtOfRail (- _output_get_2 _output_get_3))
  (bind _asbp_third_person_character (Utilities|Casting|CastToBP_ThirdPersonCharacter (Game|GetPlayerCharacter 0)))
  (Variables|Default|SetAs%20BP%20Third%20Person%20Character _asbp_third_person_character)
  (bind _output_get_4 (Variables|Default|SetFollow%20Camera (Variables|/Game/ThirdPerson/Blueprints/BP_ThirdPersonCharacter.BP_ThirdPersonCharacter_C|GetFollowCamera _asbp_third_person_character)))
  (Transformation|DetachFromComponent _output_get_4 "KeepRelative" "KeepRelative" "KeepRelative" true))

(event Collision|EventActorBeginOverlap
  (params (OtherActor :type Actor%20Object%20Reference)))

(event EventTick
  (params (DeltaSeconds :type Float%20%28single-precision%29))
  (bind _follow_camera (Variables|Default|GetFollow%20Camera))
  (bind _spline_ref (Variables|Default|GetSpline_ref))
  (Variables|Default|SetPlayer%20Value%20Y (.y (Transformation|GetWorldLocation (Variables|/Script/Engine.Character|GetMesh (Variables|Default|GetAs%20BP%20Third%20Person%20Character)))))
  (Utilities|IsValid _spline_ref
    (:Is%20Valid
      (Transformation|SetWorldLocation _follow_camera (+ (Spline|GetLocationatTime _spline_ref (Class|SplineComponent|GetTimeatDistanceAlongSpline _spline_ref (- (Variables|Default|GetPlayer%20Value%20Y) (Variables|Default|GetEnd%20Value%20Y))) "World" false) "0.000000,-500.000000,0.000000") false true)
      (Transformation|SetWorldRotation _follow_camera (Math|Rotator|MakeRotator (.roll (Class|SplineComponent|GetRotationatTime _spline_ref (Class|SplineComponent|GetTimeatDistanceAlongSpline _spline_ref (- (Variables|Default|GetPlayer%20Value%20Y) (Variables|Default|GetEnd%20Value%20Y))) "World" false)) (.pitch (Class|SplineComponent|GetRotationatTime _spline_ref (Class|SplineComponent|GetTimeatDistanceAlongSpline _spline_ref (- (Variables|Default|GetPlayer%20Value%20Y) (Variables|Default|GetEnd%20Value%20Y))) "World" false)) (+ (.yaw (Class|SplineComponent|GetRotationatTime _spline_ref (Class|SplineComponent|GetTimeatDistanceAlongSpline _spline_ref (- (Variables|Default|GetPlayer%20Value%20Y) (Variables|Default|GetEnd%20Value%20Y))) "World" false)) -9e+01)) false false))))

(fn ConstructionScript)