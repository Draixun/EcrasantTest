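; A trigger actor that switches the player's view to a different camera while BP_ThirdPersonCharacter is inside its Trigger_cam volume.
; Overlap begin blends the view target to Camera, and overlap end blends back to CameraBase, both with a timed cubic blend.
; Each switch also stores the new camera's world rotation in CameraRotation on the GameInstance_Var game instance.
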(event OnComponentBeginOverlap(Trigger_cam)
  (params (OverlappedComponent :type Primitive%20Component%20Object%20Reference) (OtherActor :type Actor%20Object%20Reference) (OtherComp :type Primitive%20Component%20Object%20Reference) (OtherBodyIndex :type Integer) (bFromSweep :type Boolean) (SweepResult :type Hit%20Result%20Structure%20%28by%20ref%29))
  (bind _camera (Variables|Default|GetCamera))
  (Utilities|Casting|CastToBP_ThirdPersonCharacter OtherActor)
  (Game|Player|SetViewTargetwithBlend (Game|GetPlayerController 0) _camera 2.0 "VTBlend_Cubic" 0.0 false)
  (bind _asgame_instance_var (Utilities|Casting|CastToGameInstance_Var (Game|GetGameInstance)))
  (Variables|/Game/BP/GameInstance/GameInstance_Var.GameInstance_Var_C|SetCamera%20Rotation _asgame_instance_var (Transformation|GetWorldRotation (Variables|/Script/Engine.CameraActor|GetCameraComponent _camera))))

(event OnComponentEndOverlap(Trigger_cam)
  (params (OverlappedComponent :type Primitive%20Component%20Object%20Reference) (OtherActor :type Actor%20Object%20Reference) (OtherComp :type Primitive%20Component%20Object%20Reference) (OtherBodyIndex :type Integer))
  (bind _camera_base (Variables|Default|GetCamera_base))
  (Utilities|Casting|CastToBP_ThirdPersonCharacter OtherActor)
  (Game|Player|SetViewTargetwithBlend (Game|GetPlayerController 0) _camera_base 2.0 "VTBlend_Cubic" 0.0 false)
  (bind _asgame_instance_var (Utilities|Casting|CastToGameInstance_Var (Game|GetGameInstance)))
  (Variables|/Game/BP/GameInstance/GameInstance_Var.GameInstance_Var_C|SetCamera%20Rotation _asgame_instance_var (Transformation|GetWorldRotation (Variables|/Script/Engine.CameraActor|GetCameraComponent _camera_base))))

(event EventBeginPlay)

(event Collision|EventActorBeginOverlap
  (params (OtherActor :type Actor%20Object%20Reference)))

(event EventTick
  (params (DeltaSeconds :type Float%20%28single-precision%29)))

(fn ConstructionScript)