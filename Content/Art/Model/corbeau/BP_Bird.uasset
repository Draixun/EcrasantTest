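; An ambient bird actor that takes flight when the player character overlaps it.
; The overlap switches the skeletal mesh to a looping fly animation, and a timeline lerps the actor to a point high above.
; Until then, a looping timer plays a move timeline that shifts the mesh around its starting location, with random offsets re-rolled every update.
; The Fly function is an empty stub.
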(event Custom|Update_move
  (bind _returnvalue (Math|Random|RandomFloatinRange 0.0 1e+02))
  (bind _pos (Variables|Default|Getpos))
  (if (not (Variables|Default|GetIsFlying))
    (Development|PrintString "cum")
    (bind _newtrack_0 (Timeline|Move Play)
      (:Update
        (Transformation|SetWorldLocation (Variables|Default|GetSkeletalMesh) (Math|Vector|Lerp(Vector) _pos (+ _pos (Math|Vector|MakeVector _returnvalue _returnvalue 0.0)) _newtrack_0) false false)))))

(event EventBeginPlay
  (Variables|Default|Setpos (Transformation|GetWorldLocation (Variables|Default|GetSkeletalMesh)))
  (Utilities|Time|SetTimerbyEvent (delegate Custom|Update_move) 0.2 true))

(event Collision|EventActorBeginOverlap
  (params (OtherActor :type Actor%20Object%20Reference))
  (Utilities|Casting|CastToBP_ThirdPersonCharacter OtherActor)
  (Variables|Default|SetStartPos (Transformation|GetActorLocation))
  (Variables|Default|SetIsFlying true)
  (Variables|Default|SetTargetPos (+ (Variables|Default|GetStartPos) "0.000000,500.000000,6000.000000"))
  (Components|Animation|PlayAnimation (Variables|Default|GetSkeletalMesh) "/Game/Art/Model/corbeau/Bird_fly.Bird_fly" true)
  (bind _alpha (Timeline|Timeline Play)
    (:Update
      (Transformation|SetActorLocation (Math|Vector|Lerp(Vector) (Variables|Default|GetStartPos) (Variables|Default|GetTargetPos) _alpha) false false))))

(event EventTick
  (params (DeltaSeconds :type Float%20%28single-precision%29)))

(fn ConstructionScript)

(fn Fly)